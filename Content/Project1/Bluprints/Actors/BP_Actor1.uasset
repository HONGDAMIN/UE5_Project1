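; BP_Actor1 is an actor whose static mesh shuttles back and forth along its local X axis.
; Tick offsets the mesh by XMultiplication each frame, without delta-time scaling, and flips the Moving flag when the accumulated offset reaches either limit.
; The construction script uses the Transform boolean to choose between AliasReference and a wireframe material for the mesh.
; Both parts print debug strings.
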(event EventTick
  (params (DeltaSeconds :type Float%20%28single-precision%29))
  (bind _xmultiplication (Variables|Default|GetXMultiplication))
  (bind _xmultiplication_2 (Variables|Default|GetXMultiplication))
  (bind _returnvalue (* _xmultiplication_2 1.0))
  (bind _returnvalue_2 (* _xmultiplication -1.0))
  ;[1 1 1] Actor Moving
  (if (Variables|Default|GetMoving)
    (Transformation|AddLocalOffset (Variables|Default|GetStaticMesh) (Math|Vector|MakeVector _returnvalue 0.0 0.0) false false)
    (Variables|Default|SetXLocalOffset (+ (Variables|Default|GetXLocalOffset) _returnvalue))
    (if (>= (Variables|Default|GetXLocalOffset) 1e+03)
      (Variables|Default|SetMoving false)
      (Development|PrintString "1000"))
    (else
      (Transformation|AddLocalOffset (Variables|Default|GetStaticMesh) (Math|Vector|MakeVector _returnvalue_2 0.0 0.0) false false)
      (Variables|Default|SetXLocalOffset (+ (Variables|Default|GetXLocalOffset) _returnvalue_2))
      (if (<= (Variables|Default|GetXLocalOffset) -1e+03)
        (Variables|Default|SetMoving true)
        (Development|PrintString "-1000")))))

(fn ConstructionScript
  ;[1 1 1] Material Transform
  (if (Variables|Default|GetTransform)
    (Rendering|Material|SetMaterial (Variables|Default|GetStaticMesh) 0 "/DatasmithContent/Materials/AliasReference.AliasReference")
    (Development|PrintString "True 변경")
    (else
      (Rendering|Material|SetMaterial (Variables|Default|GetStaticMesh) 0 "/Engine/EngineDebugMaterials/WireframeMaterial.WireframeMaterial")
      (Development|PrintString "False 변경"))))